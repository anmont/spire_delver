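; BP_DungeonInstance handles main menu display and the start of a solo game for the dungeon game.
; UIShowMainMenu creates WB_MainMenu once, caches it, adds it to the viewport and gives the first player UI-only input with a visible cursor.
; StartSoloGame opens the dungeon level by name, setting IsSoloGame to false beforehand despite the event's name.
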(event Custom|StartSoloGame
  (Variables|Default|SetIsSoloGame false)
  (Game|OpenLevel(byName) "dungeon"))

(fn UIShowMainMenu
  (bind _returnvalue (Game|GetPlayerController 0))
  (Utilities|IsValid (Variables|Default|GetWB_MainMenu)
    (:Is%20Valid
      _)
    (:Is%20Not%20Valid
      (bind _returnvalue_2 (UserInterface|CreateWidget "/Game/MainMenu/WB_MainMenu.WB_MainMenu_C" _returnvalue))
      (Variables|Default|SetWB_MainMenu _returnvalue_2)))
  (UserInterface|Viewport|AddtoViewport (Variables|Default|GetWB_MainMenu) 0)
  (Input|SetInputModeUIOnly _returnvalue 0 "DoNotLock" false)
  (Variables|/Script/Engine.PlayerController|SetbShowMouseCursor _returnvalue true)
  (return))