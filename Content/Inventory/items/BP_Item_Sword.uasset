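; BP_Item_Sword is an interactable sword item actor for the inventory system.
; FocusTarget reads the ItemID data table row from its BPCItemData and returns a "Pickup {Item}" prompt using that row's name.
; The Interact event has no logic yet, and BeginPlay, overlap and Tick are disabled stubs.
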(event EventBeginPlay
  (|CallParentFunction) ; This node is disabled and will not be called.\nDrag off pins to build functionality.
)

(event Collision|EventActorBeginOverlap
  (params (OtherActor :type Actor%20Object%20Reference))
  (|CallParentFunction OtherActor) ; This node is disabled and will not be called.\nDrag off pins to build functionality.
)

(event EventTick
  (params (DeltaSeconds :type Float%20%28single-precision%29))
  (|CallParentFunction DeltaSeconds) ; This node is disabled and will not be called.\nDrag off pins to build functionality.
)

(event EventInteract
  (params (Interactor :type BP%20First%20Person%20Character%20Object%20Reference)))

(fn ConstructionScript
  (|CallParentFunction))

(fn FocusTarget
  (bind _bpc_itemdata (Variables|Default|GetBPC_ItemData))
  (bind _itemid (Variables|/Game/Inventory/BPC_ItemData.BPC_ItemData_C|GetItemID _bpc_itemdata))
  (bind (_datatable _rowname) (Utilities|Struct|BreakDataTableRowHandle _itemid))
  (bind _returnvalue (Utilities|GetDataTableRow _datatable _rowname)
    (:then
      (return (Utilities|Text|FormatText "Pickup {Item}" (Utilities|Struct|BreakS_ItemData _returnvalue))))))