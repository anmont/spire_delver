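; Inventory component that holds a fixed-size slot array and handles the player's interaction with nearby items.
; A looping timer sphere-traces around the owner to set the target and prompt widget; IA_Interact forwards to the target's BPC_ItemData.
; Slot functions pick up, split, use (spawning an effect actor) and merge or swap between inventories, using DT_ItemData for item data.
; OnInventoryUpdated broadcasts changes; move-sound nodes are unconnected.
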(event Custom|CreateInteractMessage
  (bind _returnvalue (UserInterface|CreateWidget "/Game/Inventory/UI/WB_InteractMessage.WB_InteractMessage_C"))
  (bind _output_get (Variables|Default|SetWB_InteractMessage _returnvalue))
  (UserInterface|Viewport|AddtoViewport _output_get 0))

(event Custom|BeginInteract
  (Utilities|Time|SetTimerbyEvent (delegate Custom|UpddateInteraction) 0.2 true))

(event Custom|UpddateInteraction
  (CallFunction|Interaction))

(event Custom|UpdateInventory
  (Default|CallOnInventoryUpdated))

(event Input|EnhancedActionEvents|EnhancedInputActionIA_Interact
  (params (ActionValue :type Boolean) (ElapsedSeconds :type Float%20%28double-precision%29) (TriggeredSeconds :type Float%20%28double-precision%29) (InputAction :type Input%20Action%20Object%20Reference :default "/Game/FirstPerson/Input/Actions/IA_Interact.IA_Interact"))
  (:Started
    (bind _targetactor (Variables|Default|GetTargetActor)
      (:then
        (Utilities|IsValid (Actor|GetComponentbyClass _targetactor "/Game/Inventory/BPC_ItemData.BPC_ItemData_C")
          (:Is%20Valid
            (Class|BPIInteract|Interact(Message) (Actor|GetComponentbyClass _targetactor "/Game/Inventory/BPC_ItemData.BPC_ItemData_C") (.AsBP%20First%20Person%20Character (Utilities|Casting|CastToBP_FirstPersonCharacter (Game|GetPlayerCharacter 0)))))))
      (:else))))

(event EventBeginPlay
  (Utilities|Array|Resize (Variables|Default|GetItemSlots) (Variables|Default|GetInventorySize)))

(fn PrintInventory
  (for (_array_element _array_index) (Variables|Default|GetItemSlots)
    (Development|PrintString (Utilities|String|Append (Utilities|String|ToString(Integer) _array_index) ":" (Utilities|String|ToString(Name) (.itemID (Utilities|Struct|BreakS_ItemSlot _array_element))) "=" (Utilities|String|ToString(Integer) (.itemQty (Utilities|Struct|BreakS_ItemSlot _array_element)))))))

(fn Interaction
  (bind _returnvalue (Components|GetOwner))
  (bind _returnvalue_2 (Transformation|GetActorLocation _returnvalue))
  (bind (_outhit _returnvalue_3) (Collision|SphereTraceByChannel _returnvalue_2 _returnvalue_2 (Variables|Default|GetInteractRadius) "TraceTypeQuery3" false (Utilities|Array|MakeArray (Components|GetOwner)) "None"))
  (if _returnvalue_3
    (if (!= (.HitActor (Collision|BreakHitResult _outhit)) (Variables|Default|GetTargetActor))
      (bind _output_get (Variables|Default|SetTargetActor (.HitActor (Collision|BreakHitResult _outhit))))
      (bind _message (Class|BPIInteract|FocusTarget(Message) _output_get))
      (Default|SetInteractMessage (Variables|Default|GetWB_InteractMessage) _message))
    (else
      (Variables|Default|SetTargetActor 0)
      (Default|SetInteractMessage (Variables|Default|GetWB_InteractMessage)))))

(fn Pickup
  (params (ItemIDD :type Name) (ItemQty :type Integer))
  (bind (_success _array_index) (CallFunction|AnySlotAvailable))
  (bind _output_get (LocalVariables|SetLocal_ItemQty ItemQty))
  (while (and (> _output_get 0) (not (LocalVariables|GetLocal_IsFull)))
    (bind (_success_2 _array_index_2) (CallFunction|FindSlot ItemIDD))
    (if _success_2
      (CallFunction|AddtoStack _array_index_2 1)
      (Math|Integer|DecrementInt (LocalVariables|GetLocal_ItemQty)
        (:%20%20
          (return true 0)))
      (elif _success
        (CallFunction|CreateNewStack ItemIDD 1 _array_index)
        (Math|Integer|DecrementInt (LocalVariables|GetLocal_ItemQty)
          (:%20%20
            (return true 0)))
        (else
          (LocalVariables|SetLocal_IsFull true)))))
  (return (not (LocalVariables|GetLocal_IsFull)) (LocalVariables|GetLocal_ItemQty)))

(fn FindSlot
  (params (ItemID :type Name))
  (for (_array_element _array_index) (Variables|Default|GetItemSlots)
    (if (and (== ItemID (.itemID (Utilities|Struct|BreakS_ItemSlot _array_element))) (< (.itemQty (Utilities|Struct|BreakS_ItemSlot _array_element)) (CallFunction|GetMaxStackSize ItemID)))
      (return true _array_index)))
  (return false -1))

(fn GetMaxStackSize
  (params (ItemID :type Name))
  (bind _returnvalue (Utilities|GetDataTableRow "/Game/Inventory/itemData/DT_ItemData.DT_ItemData" ItemID)
    (:then
      (return (Utilities|Struct|BreakS_ItemData _returnvalue)))))

(fn AddtoStack
  (params (Index :type Integer) (ItemQty :type Integer))
  (bind _itemslots (Variables|Default|GetItemSlots))
  (bind _output (Utilities|Array|Get(acopy) _itemslots Index))
  (Utilities|Array|SetArrayElem (Variables|Default|GetItemSlots) Index (Utilities|Struct|MakeS_ItemSlot (.itemid _output) (+ ItemQty (.itemqty _output)))))

(fn AnySlotAvailable
  (for (_array_element _array_index) (Variables|Default|GetItemSlots)
    (if (== (.itemQty (Utilities|Struct|BreakS_ItemSlot _array_element)) 0)
      (return true _array_index)))
  (return false -1))

(fn CreateNewStack
  (params (ItemID :type Name) (ItemQty :type Integer) (Index :type Integer))
  (Utilities|Array|SetArrayElem (Variables|Default|GetItemSlots) Index (Utilities|Struct|MakeS_ItemSlot ItemID ItemQty)))

(fn SplitStack
  (params (Intex :type Integer))
  (bind (_success _array_index) (CallFunction|AnySlotAvailable))
  (bind _itemslots (Variables|Default|GetItemSlots))
  (bind _output (Utilities|Array|Get(acopy) _itemslots Intex))
  (LocalVariables|SetLocalItemIDD (.itemid _output))
  (LocalVariables|SetLocalQuantity (.itemqty _output))
  (Utilities|FlowControl|Sequence
    (:then_0
      (if (not (== (LocalVariables|GetLocalQuantity) 1))
        (if _success
          (LocalVariables|SetLocalSplitQty (/ (LocalVariables|GetLocalQuantity) 2))
          (Utilities|Array|SetArrayElem (Variables|Default|GetItemSlots) _array_index (Utilities|Struct|MakeS_ItemSlot (LocalVariables|GetLocalItemIDD) (LocalVariables|GetLocalSplitQty)))
          (Utilities|Array|SetArrayElem (Variables|Default|GetItemSlots) Intex (Utilities|Struct|MakeS_ItemSlot (LocalVariables|GetLocalItemIDD) (- (LocalVariables|GetLocalQuantity) (LocalVariables|GetLocalSplitQty))))
          (CallFunction|UpdateInventory))))
    (:then_1
      (bind _returnvalue (Utilities|GetDataTableRow "/Game/Inventory/itemData/DT_ItemData.DT_ItemData" (LocalVariables|GetLocalItemIDD))))))

(fn UseItem
  (params (Index :type Integer))
  (bind _itemslots (Variables|Default|GetItemSlots))
  (bind _output (Utilities|Array|Get(acopy) _itemslots))
  (LocalVariables|SetLocalItemID (.itemid _output))
  (LocalVariables|SetLocalQty (.itemqty _output))
  (Utilities|FlowControl|Sequence
    (:then_0
      (if (== (LocalVariables|GetLocalQty) 1)
        (Utilities|Array|SetArrayElem (Variables|Default|GetItemSlots) Index (Utilities|Struct|MakeS_ItemSlot "None" 0))
        (else
          (CallFunction|UpdateStack Index 1)))
      (Game|SpawnActorfromClass (Utilities|Struct|BreakS_ItemData (CallFunction|GetItemData (LocalVariables|GetLocalItemID))) (CallFunction|GetDropLocation) "Undefined" "MultiplyWithRoot" 0 "Hello" 0)
      (CallFunction|UpdateInventory))
    (:then_1
      (bind _returnvalue (Utilities|GetDataTableRow "/Game/Inventory/itemData/DT_ItemData.DT_ItemData" (LocalVariables|GetLocalItemID))))))

(fn UpdateStack
  (params (Index :type Integer) (Quantity :type Integer))
  (bind _itemslots (Variables|Default|GetItemSlots))
  (bind _output (Utilities|Array|Get(acopy) _itemslots Index))
  (Utilities|Struct|SetmembersinS_ItemSlot _output (- (.itemQty (Utilities|Struct|BreakS_ItemSlot _output)) Quantity)))

(fn GetDropLocation
  (bind _returnvalue (Components|GetOwner))
  (return (+ (Transformation|GetActorLocation _returnvalue) (* (Math|Random|RandomUnitVectorinConeinDegrees (Transformation|GetActorForwardVector _returnvalue) 55.0) 1.2e+02))))

(fn GetItemData
  (params (ItemID :type Name))
  (bind _returnvalue (Utilities|GetDataTableRow "/Game/Inventory/itemData/DT_ItemData.DT_ItemData" ItemID)
    (:then
      (return _returnvalue))))

(fn TransferSlot
  (params (Index :type Integer) (SourceIndex :type Integer) (SourceInventory :type BPC%20Inventory%20Object%20Reference))
  (bind _itemslots (Variables|Default|GetItemSlots))
  (bind _output (Utilities|Array|Get(acopy) _itemslots Index))
  (Utilities|FlowControl|Sequence
    (:then_0
      (LocalVariables|SetLocal_SourceSlot (Utilities|Array|Get(acopy) (Variables|BPC_Inventory_C|GetItemSlots SourceInventory) SourceIndex))
      (Development|PrintString (Utilities|String|Append "Do Strings Match" (Utilities|String|ToString(Boolean) (== (.itemID (Utilities|Struct|BreakS_ItemSlot (Utilities|Array|Get(acopy) (Variables|Default|GetItemSlots) Index))) (Utilities|Struct|BreakS_ItemSlot (LocalVariables|GetLocal_SourceSlot))))))
      (if (== (.itemID (Utilities|Struct|BreakS_ItemSlot (Utilities|Array|Get(acopy) (Variables|Default|GetItemSlots) Index))) (Utilities|Struct|BreakS_ItemSlot (LocalVariables|GetLocal_SourceSlot)))
        (CallFunction|CreateNewStack SourceInventory (select (> (Math|Integer|Clamp(Integer) (- (+ (.itemQty (Utilities|Struct|BreakS_ItemSlot (Utilities|Array|Get(acopy) (Variables|Default|GetItemSlots) Index))) (.itemQty (Utilities|Struct|BreakS_ItemSlot (LocalVariables|GetLocal_SourceSlot)))) (CallFunction|GetMaxStackSize (.itemID (Utilities|Struct|BreakS_ItemSlot (LocalVariables|GetLocal_SourceSlot))))) 0 (CallFunction|GetMaxStackSize (.itemID (Utilities|Struct|BreakS_ItemSlot (LocalVariables|GetLocal_SourceSlot))))) 0) (Utilities|Struct|BreakS_ItemSlot (LocalVariables|GetLocal_SourceSlot)) "None") (Math|Integer|Clamp(Integer) (- (+ (.itemQty (Utilities|Struct|BreakS_ItemSlot (Utilities|Array|Get(acopy) (Variables|Default|GetItemSlots) Index))) (.itemQty (Utilities|Struct|BreakS_ItemSlot (LocalVariables|GetLocal_SourceSlot)))) (CallFunction|GetMaxStackSize (.itemID (Utilities|Struct|BreakS_ItemSlot (LocalVariables|GetLocal_SourceSlot))))) 0 (CallFunction|GetMaxStackSize (.itemID (Utilities|Struct|BreakS_ItemSlot (LocalVariables|GetLocal_SourceSlot))))) SourceIndex)
        (CallFunction|CreateNewStack (.itemID (Utilities|Struct|BreakS_ItemSlot (LocalVariables|GetLocal_SourceSlot))) (Math|Integer|Clamp(Integer) (+ (Utilities|Struct|BreakS_ItemSlot (Utilities|Array|Get(acopy) (Variables|Default|GetItemSlots) Index)) (.itemQty (Utilities|Struct|BreakS_ItemSlot (LocalVariables|GetLocal_SourceSlot)))) 0 (CallFunction|GetMaxStackSize (.itemID (Utilities|Struct|BreakS_ItemSlot (LocalVariables|GetLocal_SourceSlot))))) Index)
        (else
          (CallFunction|CreateNewStack SourceInventory (.itemid _output) (.itemqty _output) SourceIndex)
          (CallFunction|CreateNewStack (.itemID (Utilities|Struct|BreakS_ItemSlot (LocalVariables|GetLocal_SourceSlot))) (.itemQty (Utilities|Struct|BreakS_ItemSlot (LocalVariables|GetLocal_SourceSlot))) Index)
          (CallFunction|UpdateInventory))))
    (:then_1
      (bind _returnvalue (Utilities|GetDataTableRow "/Game/Inventory/itemData/DT_ItemData.DT_ItemData" (Utilities|Struct|BreakS_ItemSlot (Utilities|Array|Get(acopy) (Variables|Default|GetItemSlots) Index)))))))