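; BPC_Stats is a stats Blueprint that holds Health and Gray Mana values.
; IncreaseValue switches on the chosen stat and adds the given amount to it, with no clamping applied.
; After a Health change it calls Die if Health is zero or below, but the Die event is still empty.
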(event Custom|Die)

(fn IncreaseValue
  (params (Stat :type E_Stats%20Enum :default "NewEnumerator0") (Value :type Float%20%28double-precision%29))
  (switch Utilities|FlowControl|Switch|SwitchonE_Stats Stat
    (:NewEnumerator0
      (Variables|Default|SetHealth (+ (Variables|Default|GetHealth) Value))
      (Utilities|FlowControl|Sequence
        (:then_0
          (if (<= (Variables|Default|GetHealth) 0.0)
            (CallFunction|Die)))))
    (:NewEnumerator1
      (Variables|Default|SetGrayMana (+ (Variables|Default|GetGrayMana) Value)))))